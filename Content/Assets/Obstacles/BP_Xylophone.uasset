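; BP_Xylophone is an interactable obstacle that opens a xylophone widget for the player.
; Sphere overlap events cache the first-person character and toggle the Unlock component's visibility.
; While overlapping, Tick polls the player's Interacting flag behind a short Delay, then creates the widget, shows the cursor and pauses the game.
; Once Completed is true, Tick destroys the sphere and hides Unlock, ending interaction.
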(event OnComponentBeginOverlap(Sphere)
  (params (OverlappedComponent :type Primitive%20Component%20Object%20Reference) (OtherActor :type Actor%20Object%20Reference) (OtherComp :type Primitive%20Component%20Object%20Reference) (OtherBodyIndex :type Integer) (bFromSweep :type Boolean) (SweepResult :type Hit%20Result%20Structure%20%28by%20ref%29))
  (bind _asbp_first_person_character (Utilities|Casting|CastToBP_FirstPersonCharacter OtherActor))
  (Variables|Default|SetPlayer _asbp_first_person_character)
  (Variables|Default|SetOverlapping true)
  (Development|SetHiddeninGame (Variables|Default|GetUnlock) false true))

(event OnComponentEndOverlap(Sphere)
  (params (OverlappedComponent :type Primitive%20Component%20Object%20Reference) (OtherActor :type Actor%20Object%20Reference) (OtherComp :type Primitive%20Component%20Object%20Reference) (OtherBodyIndex :type Integer))
  (Variables|Default|SetOverlapping false)
  (Development|SetHiddeninGame (Variables|Default|GetUnlock) true true))

(event EventTick
  (params (DeltaSeconds :type Float%20%28single-precision%29))
  (bind _returnvalue (Game|GetPlayerController 0))
  (if (Variables|Default|Getcompleted)
    (bind _sphere (Variables|Default|GetSphere)
      (:then
        (Components|DestroyComponent _sphere)
        (Development|SetHiddeninGame (Variables|Default|GetUnlock) true true))
      (:else))
    (elif (Variables|Default|GetOverlapping)
      (Utilities|FlowControl|Delay 0.1)
      (if (Variables|/Game/FirstPerson/Blueprints/BP_FirstPersonCharacter.BP_FirstPersonCharacter_C|GetInteracting (Variables|Default|GetPlayer))
        (bind _returnvalue_2 (UserInterface|CreateWidget "/Game/UI/Xylophone/Xylophone.Xylophone_C" _returnvalue))
        (UserInterface|Viewport|AddtoViewport _returnvalue_2 0)
        (Variables|/Script/Engine.PlayerController|SetbShowMouseCursor _returnvalue true)
        (Game|SetGamePaused true)))))

(fn ConstructionScript
  (|CallParentFunction))