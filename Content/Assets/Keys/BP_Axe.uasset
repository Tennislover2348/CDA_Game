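; BP_Axe is a pickup item that sets HasAxe on the first-person character, then runs the parent pickup logic.
; Its sphere overlap stores the player, reveals the Interact prompt and lights GlowKey2 blue through the Colors parameter collection.
; Tick polls the player's Interacting flag, with CanPickup armed by a short delay while not interacting.
; Overlap and pickup logic only run while the collection's Green parameter is zero.
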(event OnComponentBeginOverlap(Sphere)
  (params (OverlappedComponent :type Primitive%20Component%20Object%20Reference) (OtherActor :type Actor%20Object%20Reference) (OtherComp :type Primitive%20Component%20Object%20Reference) (OtherBodyIndex :type Integer) (bFromSweep :type Boolean) (SweepResult :type Hit%20Result%20Structure%20%28by%20ref%29))
  (bind _returnvalue (Rendering|Material|GetScalarParameterValue "/Game/Colors/Colors.Colors" "Green" :!class /Script/Engine.KismetMaterialLibrary))
  (if (== _returnvalue 0.0)
    (bind _asbp_first_person_character (Utilities|Casting|CastToBP_FirstPersonCharacter OtherActor))
    (Variables|Default|SetPlayer _asbp_first_person_character)
    (Variables|Default|SetOverlapping true)
    (Development|SetHiddeninGame (Variables|Default|GetInteract) false true)
    (Rendering|Material|SetVectorParameterValue "/Game/Colors/Colors.Colors" "GlowKey2" (Utilities|Struct|MakeLinearColor 0.0 0.0 1.0 1.0) :!class /Script/Engine.KismetMaterialLibrary)))

(event OnComponentEndOverlap(Sphere)
  (params (OverlappedComponent :type Primitive%20Component%20Object%20Reference) (OtherActor :type Actor%20Object%20Reference) (OtherComp :type Primitive%20Component%20Object%20Reference) (OtherBodyIndex :type Integer))
  (bind _returnvalue (Rendering|Material|GetScalarParameterValue "/Game/Colors/Colors.Colors" "Green" :!class /Script/Engine.KismetMaterialLibrary))
  (if (== _returnvalue 0.0)
    (Variables|Default|SetOverlapping false)
    (Development|SetHiddeninGame (Variables|Default|GetInteract) true true)
    (Rendering|Material|SetVectorParameterValue "/Game/Colors/Colors.Colors" "GlowKey2" (Utilities|Struct|MakeLinearColor 0.0 0.0 0.0 0.0) :!class /Script/Engine.KismetMaterialLibrary)))

(event EventBeginPlay
  (|CallParentFunction))

(event Collision|EventActorBeginOverlap
  (params (OtherActor :type Actor%20Object%20Reference))
  (bind _returnvalue (Rendering|Material|GetScalarParameterValue "/Game/Colors/Colors.Colors" "Green" :!class /Script/Engine.KismetMaterialLibrary))
  (if (== _returnvalue 0.0)
    (|CallParentFunction 0)))

(event EventTick
  (params (DeltaSeconds :type Float%20%28single-precision%29))
  (bind _player (Variables|Default|GetPlayer))
  (bind _returnvalue (Rendering|Material|GetScalarParameterValue "/Game/Colors/Colors.Colors" "Green" :!class /Script/Engine.KismetMaterialLibrary))
  (if (== _returnvalue 0.0)
    (if (Variables|Default|GetOverlapping)
      (if (Variables|/Game/FirstPerson/Blueprints/BP_FirstPersonCharacter.BP_FirstPersonCharacter_C|GetInteracting _player)
        (if (Variables|Default|GetCanPickup)
          (Variables|/Game/FirstPerson/Blueprints/BP_FirstPersonCharacter.BP_FirstPersonCharacter_C|SetInteracting _player false)
          (CallFunction|ItemPickup))
        (else
          (Utilities|FlowControl|Delay 0.5)
          (Variables|Default|SetCanPickup true))))))

(fn ConstructionScript
  (|CallParentFunction))

(fn ItemPickup
  (Variables|/Game/FirstPerson/Blueprints/BP_FirstPersonCharacter.BP_FirstPersonCharacter_C|SetHasAxe (Variables|Default|GetPlayer) true)
  (|CallParentFunction))