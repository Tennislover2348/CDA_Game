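; BP_Interactable is an item actor that the first-person character picks up by interacting while in range.
; A Sphere overlap caches the BP_FirstPersonCharacter and toggles the Interact prompt's visibility on enter and exit.
; While overlapping, Tick polls the player's Interacting flag and calls ItemPickup, which passes the item to the player's own ItemPickup and then destroys the actor.
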(event OnComponentBeginOverlap(Sphere)
  (params (OverlappedComponent :type Primitive%20Component%20Object%20Reference) (OtherActor :type Actor%20Object%20Reference) (OtherComp :type Primitive%20Component%20Object%20Reference) (OtherBodyIndex :type Integer) (bFromSweep :type Boolean) (SweepResult :type Hit%20Result%20Structure%20%28by%20ref%29))
  (bind _asbp_first_person_character (Utilities|Casting|CastToBP_FirstPersonCharacter OtherActor))
  (Variables|Default|SetPlayer _asbp_first_person_character)
  (Variables|Default|SetOverlapping true)
  (Development|SetHiddeninGame (Variables|Default|GetInteract) false true))

(event OnComponentEndOverlap(Sphere)
  (params (OverlappedComponent :type Primitive%20Component%20Object%20Reference) (OtherActor :type Actor%20Object%20Reference) (OtherComp :type Primitive%20Component%20Object%20Reference) (OtherBodyIndex :type Integer))
  (Variables|Default|SetOverlapping false)
  (Development|SetHiddeninGame (Variables|Default|GetInteract) true true))

(event EventBeginPlay)

(event Collision|EventActorBeginOverlap
  (params (OtherActor :type Actor%20Object%20Reference)))

(event EventTick
  (params (DeltaSeconds :type Float%20%28single-precision%29))
  (if (Variables|Default|GetOverlapping)
    (if (Variables|/Game/FirstPerson/Blueprints/BP_FirstPersonCharacter.BP_FirstPersonCharacter_C|GetInteracting (Variables|Default|GetPlayer))
      (CallFunction|ItemPickup))))

(fn ConstructionScript)

(fn ItemPickup
  (Default|ItemPickup (Variables|Default|GetPlayer) self)
  (Actor|DestroyActor))